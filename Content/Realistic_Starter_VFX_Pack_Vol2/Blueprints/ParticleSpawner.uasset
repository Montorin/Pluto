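; ParticleSpawner is an actor that plays a configurable particle effect at its placed location.
; On BeginPlay it applies a world scale to its root and assigns the Effect template to its VFX component.
; It activates the effect, waits an interval, then either deactivates and replays it when looping or destroys itself.
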(event `self.ReceiveBeginPlay`
  (bind _vfx (`self.VFX`))
  (`SceneComponent.SetWorldScale3D` (`self.DefaultSceneRoot`) (`self.scale`))
  (`ParticleSystemComponent.SetTemplate` (`self.VFX`) (`self.effect`))
  (`/Engine/EditorBlueprintResources/StandardMacros.IsValid` (`self.effect`) :!label _label
    (:`Is Valid`
      (`ActorComponent.Activate` _vfx false)
      (`KismetSystemLibrary.Delay` (`self.interval`))
      (if (`self.isLoop`)
        (`ActorComponent.Deactivate` _vfx)
        (goto _label)
        (else
          (`self.K2_DestroyActor`))))))

(fn `UserConstructionScript`)