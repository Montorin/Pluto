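; Anim notify state that sets an action state on the owner's AC_EasyComboBuffering component for the length of an animation window.
; On begin it writes its ActionState to the component.
; On end it resets to the first enum value only if the component still holds that same state, so a newer state is not overwritten.
; The notify's display name comes from the chosen ActionState enum.
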(fn `GetNotifyName`
  (returns (ReturnValue :type String))
  (return (`|GetEnumeratorNameAsString` (`self.ActionState`))))

(fn `Received_NotifyBegin`
  (params (MeshComp :type "SkeletalMeshComponent Object Reference") (Animation :type "AnimSequenceBase Object Reference") (TotalDuration :type "Float (single-precision)") (EventReference :type "AnimNotifyEventReference Structure (by ref)"))
  (returns (ReturnValue :type Boolean))
  (bind _returnvalue (`Actor.GetComponentByClass` (`ActorComponent.GetOwner` MeshComp) "/Game/EasyComboBuffering/ECB_Component/BluePrints/AC_EasyComboBuffering.AC_EasyComboBuffering_C"))
  (`/Engine/EditorBlueprintResources/StandardMacros.IsValid` _returnvalue
    (:`Is Valid`
      (`/Game/EasyComboBuffering/ECB_Component/BluePrints/AC_EasyComboBuffering.SetActionState` _returnvalue (`self.ActionState`))
      (return true))
    (:`Is Not Valid`
      (return false))))

(fn `Received_NotifyEnd`
  (params (MeshComp :type "SkeletalMeshComponent Object Reference") (Animation :type "AnimSequenceBase Object Reference") (EventReference :type "AnimNotifyEventReference Structure (by ref)"))
  (returns (ReturnValue :type Boolean))
  (bind _returnvalue (`Actor.GetComponentByClass` (`ActorComponent.GetOwner` MeshComp) "/Game/EasyComboBuffering/ECB_Component/BluePrints/AC_EasyComboBuffering.AC_EasyComboBuffering_C"))
  (`/Engine/EditorBlueprintResources/StandardMacros.IsValid` _returnvalue
    (:`Is Valid`
      (if (== (`/Game/EasyComboBuffering/ECB_Component/BluePrints/AC_EasyComboBuffering.GetActionState` _returnvalue) (`self.ActionState`))
        (`/Game/EasyComboBuffering/ECB_Component/BluePrints/AC_EasyComboBuffering.SetActionState` _returnvalue "NewEnumerator0")
        (return true)))
    (:`Is Not Valid`
      (return false))))