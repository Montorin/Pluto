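; LevelManager is a level actor that sets up the main menu and plays the level's background music.
; On BeginPlay, if IsMainMenu is set, it shows the mouse cursor and creates the MainMenu_UI widget, passing itself as a reference.
; It then sets the music component's volume multiplier from BP_GameInstance's VoiceMultiplier and starts BackgroundMusic.
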(event `self.ReceiveBeginPlay`
  (bind _musicplayercomponenet (`self.MusicPlayerComponenet`))
  (if (`self.isMainMenu`)
    (set `PlayerController.bShowMouseCursor` true (`GameplayStatics.GetPlayerController` 0))
    (bind _returnvalue (`|CreateWidget` "/Game/UI/MainMenu_UI.MainMenu_UI_C"))
    (set `/Game/UI/MainMenu_UI.levelManager` self _returnvalue)
    (`UserWidget.AddToViewport` _returnvalue 0))
  (bind _asbp_game_instance (cast `/Game/Blueprints/BP_GameInstance` (`GameplayStatics.GetGameInstance`)))
  (set `AudioComponent.VolumeMultiplier` (`/Game/Blueprints/BP_GameInstance.voiceMultiplier` _asbp_game_instance) _musicplayercomponenet)
  (`AudioComponent.SetSound` _musicplayercomponenet (`self.backgroundMusic`))
  (`AudioComponent.Play` _musicplayercomponenet 0.0))

(fn `UserConstructionScript`)