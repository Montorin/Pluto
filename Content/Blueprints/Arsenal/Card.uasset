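; Base-style Card Blueprint in the Arsenal folder for a castable spell with an energy cost.
; ActivateSpell is an empty event, and CheckCast compares supplied energy to Cost, returning the remaining energy and a can-cast flag when affordable.
; An unconnected graph fragment, meant to set the Player reference, tries casting player characters 1 to 3 to Player_BP and never runs.
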(event `ActivateSpell`)

(fn `Check Cast`
  (params (energy :type Integer))
  (returns (energyLeft :type Integer) (`canCast?` :type Boolean))
  (bind _cost (`self.Cost`))
  (bind _returnvalue (>= energy _cost))
  (if _returnvalue
    (return (- energy _cost) _returnvalue)))

(fn `UserConstructionScript`)